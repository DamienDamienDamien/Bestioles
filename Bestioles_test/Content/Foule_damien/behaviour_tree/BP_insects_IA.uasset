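; BP_insects_IA is an AI-controlled insect that tilts its mesh to the ground and reacts to apples.
; Each tick, a downward trace along the mesh's up vector gives the floor normal, from which slope angles smoothly drive pitch and roll.
; Overlapping a Pomme_trou clears the "is Hurt" Blackboard key, with debug prints.
; BeginPlay caches the player character and binds that overlap.
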(event `self.ReceiveBeginPlay`
  (bind _asbp_third_person_character_damien (cast `/Game/Foule_damien/BP_ThirdPersonCharacter_damien` (`GameplayStatics.GetPlayerCharacter` 0)))
  (set `self.char` _asbp_third_person_character_damien)
  (add `self.OnActorBeginOverlap` (delegate `OnActorBeginOverlap_Event`)))

(event `self.ReceiveTick`
  (params (DeltaSeconds :type "Float (single-precision)"))
  (`self.BAlign to floor` DeltaSeconds))

(event `BAlign to floor`
  (params (delta :type "Float (double-precision)"))
  (bind _staticmesh (`self.StaticMesh`))
  (bind _returnvalue (`SceneComponent.K2_GetComponentLocation` _staticmesh))
  (bind _returnvalue_2 (`SceneComponent.K2_GetComponentRotation` (`self.StaticMesh`)))
  ;[0.4609 1 0.3646 0.5] Raycast entre le character et le sol pour adapter sa rotation
  (bind _outhit (`KismetSystemLibrary.LineTraceSingle` :`Start` _returnvalue :`End` (- _returnvalue (* (`SceneComponent.GetUpVector` _staticmesh) 100.0)) :`TraceChannel` "TraceTypeQuery1" :`TraceColor` (struct :`R` 0.11944 :`B` 1.0 :`A` 1.0)))
  (bind (_outslopepitchdegreeangle _outsloperolldegreeangle) (`KismetMathLibrary.GetSlopeDegreeAngles` (`self.GetActorRightVector`) (`.ImpactNormal` (`GameplayStatics.BreakHitResult` _outhit)) (`self.GetActorUpVector`)))
  (bind _result (`/Engine/EditorBlueprintResources/StandardMacros.NegateFloat` _outslopepitchdegreeangle)
    (:`  `
      (bind _result_2 (`/Engine/EditorBlueprintResources/StandardMacros.NegateFloat` _outsloperolldegreeangle)
        (:`  `
          (`SceneComponent.K2_SetWorldRotation` (`self.StaticMesh`) (`KismetMathLibrary.RInterpTo` _returnvalue_2 (`KismetMathLibrary.MakeRotator` _result _result_2 (.yaw _returnvalue_2)) delta 10.0) false false))))))

(event `OnActorBeginOverlap_Event` :!signature `self.OnActorBeginOverlap`
  (params (OverlappedActor :type "Actor Object Reference") (OtherActor :type "Actor Object Reference"))
  (`KismetSystemLibrary.PrintString` (`KismetSystemLibrary.GetDisplayName` OtherActor))
  (cast `/Game/Foule_damien/Pomme/pomme_trou/Pomme_trou` OtherActor)
  (`KismetSystemLibrary.PrintString` "pomme")
  (`BlackboardComponent.SetValueAsBool` (`AIBlueprintHelperLibrary.GetBlackboard` (`AIBlueprintHelperLibrary.GetAIController` self)) "is Hurt" false))

(fn `UserConstructionScript`)