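; BP_character is a click-to-move player character, apparently a goose, that shows the mouse cursor on BeginPlay.
; A left click runs GooseMovement, which deprojects the cursor into the world and line traces on the Visibility channel.
; On a hit, it stores the point in Loc, spawns a BP_location_circle marker there at a fixed height, and sends the player controller there via SimpleMoveToLocation.
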(event `ShowMouseCursor`
  (set `PlayerController.bShowMouseCursor` true (`GameplayStatics.GetPlayerController` 0)))

(event `self.ReceiveBeginPlay`
  (`self.ShowMouseCursor`))

(event `GooseMovement`
  (bind (_worldlocation _worlddirection) (`PlayerController.DeprojectMousePositionToWorld` (`GameplayStatics.GetPlayerController` 0)))
  (bind (_outhit _returnvalue) (`KismetSystemLibrary.LineTraceSingle` _worldlocation (+ _worldlocation (* _worlddirection 5000)) "TraceTypeQuery1"))
  (if _returnvalue
    (bind (_bblockinghit _binitialoverlap _time _distance _location) (`GameplayStatics.BreakHitResult` _outhit))
    (set `self.loc` _location)
    (`|SpawnActorFromClass` "/Game/Foule/BP_location_circle.BP_location_circle_C" (`KismetMathLibrary.MakeTransform` (`KismetMathLibrary.MakeVector` (.x _location) (.y _location) 3.0)) "Undefined" "MultiplyWithRoot" null null)
    (`AIBlueprintHelperLibrary.SimpleMoveToLocation` (`GameplayStatics.GetPlayerController` 0) _location)))

(event `Key|LeftMouseButton`
  (params (Key :type "Key Structure"))
  (:`Pressed`
    (`self.GooseMovement`)))

(fn `UserConstructionScript`)