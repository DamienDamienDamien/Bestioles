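; BP_spawn is a spawner Blueprint that creates an IA_NPC actor when play begins.
; BeginPlay calls EnableInput, then runs a spawn loop currently set to a single iteration.
; Each spawn gets a random X/Y around the world origin at a fixed height, independent of the spawner's own location.
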(event `self.ReceiveBeginPlay`
  (`self.EnableInput` null)
  (for _ (range 1 2)
    (`|SpawnActorFromClass` "/Game/Foule/IA/IA_NPC.IA_NPC_C" (`KismetMathLibrary.MakeTransform` (`KismetMathLibrary.MakeVector` (* (- (* (`KismetMathLibrary.RandomFloat`) 2.0) 1.0) 100.0) (* (- (* (`KismetMathLibrary.RandomFloat`) 2.0) 1.0) 100.0) 90.0)) "Undefined" "MultiplyWithRoot" null null)))

(fn `UserConstructionScript`)