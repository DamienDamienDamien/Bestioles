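; Apple actor that, on BeginPlay, spawns half-scale IA_NPC_worm actors around itself, one per NbInsecte read from the level's Spawning actor.
; It estimates a radius from its bounds origin to a closest collision point, slightly inset, then places worms by cosine and sine of an index-based angle.
; Height climbs by a fixed step independently of the apple's Z.
; Positions are stored in ListPosition, printed and shown with debug drawing.
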(event `self.ReceiveBeginPlay`
  (bind (_origin _boxextent) (`self.GetActorBounds` false))
  (bind _outpointonbody (`PrimitiveComponent.GetClosestPointOnCollision` (`self.StaticMesh`) _boxextent "None"))
  (bind _returnvalue (+ (`self.z`) (`self.offset`)))
  (bind _returnvalue_2 (+ (.x (`self.pomme location`)) (`self.x`)))
  (bind _returnvalue_3 (+ (.y (`self.pomme location`)) (`self.y`)))
  (bind _returnvalue_4 (`GameplayStatics.GetActorOfClass` "/Game/Foule/pas_mal/spawning.spawning_C"))
  (set `self.pomme location` (`self.K2_GetActorLocation`))
  (set `self.pomme bounds` _boxextent)
  (set `self.pomme taille` (.z (`self.GetActorScale3D`)))
  (`KismetSystemLibrary.DrawDebugPoint` (`KismetMathLibrary.MakeVector` (.x _origin) (.y _origin) 130.0) 20.0 (struct :`R` 1.0 :`G` 0.731984 :`A` 1.0) 1000.0)
  (set `self.pomme rayon` (- (`KismetMathLibrary.Distance2D` (`KismetMathLibrary.Conv_VectorToVector2D` _origin) (`KismetMathLibrary.Conv_VectorToVector2D` _outpointonbody)) 10.0))
  (`KismetSystemLibrary.DrawDebugLine` (`KismetMathLibrary.MakeVector` (.x _origin) (.y _origin) 130.0) (`KismetMathLibrary.MakeVector` (.x _outpointonbody) (.y _outpointonbody) 130.0) (struct :`R` 1.0 :`B` 0.407399 :`A` 1.0) 1000.0 20.0)
  (bind _nb_insecte (`/Game/Foule/pas_mal/spawning.Nb insecte` _returnvalue_4))
  (for _index (range _nb_insecte)
    (set `self.angle` (* (/ (* _index 2) _nb_insecte) (* 2.0 (`KismetMathLibrary.GetPI`))))
    (set `self.x` (* (`self.pomme rayon`) (`KismetMathLibrary.Cos` (`self.angle`))))
    (set `self.y` (* (`self.pomme rayon`) (`KismetMathLibrary.Sin` (`self.angle`))))
    (set `self.offset` (+ (`self.offset`) 8.0))
    (bind _output_get (set `self.i` (`KismetMathLibrary.MakeVector` _returnvalue_2 _returnvalue_3 _returnvalue)))
    (`KismetSystemLibrary.DrawDebugPoint` (`KismetMathLibrary.MakeVector` _returnvalue_2 _returnvalue_3 _returnvalue) 20.0 (struct :`G` 0.02487 :`B` 1.0 :`A` 1.0) 1000.0)
    (`KismetArrayLibrary.Array_Add` (`self.list position`) _output_get)
    (`KismetSystemLibrary.PrintString` (`KismetStringLibrary.Conv_VectorToString` _output_get))
    (`|SpawnActorFromClass` "/Game/Foule/pas_mal/IA_NPC/IA_NPC_worm.IA_NPC_worm_C" (`KismetMathLibrary.MakeTransform` _output_get (struct) (0.5 0.5 0.5)) "Undefined" "MultiplyWithRoot" null null)))

(fn `UserConstructionScript`)