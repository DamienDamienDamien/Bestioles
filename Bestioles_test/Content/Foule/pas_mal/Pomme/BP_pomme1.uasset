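; Apple actor that hands worm NPCs target positions on itself and triggers their eating.
; At BeginPlay, PostPCG sets its instanced mesh components to a worm mesh and records one instance location from each, using the component's index as instance index.
; Pressing A walks the Spawning actor's InsectList, assigns each worm the location at its matching index, then calls CallEat.
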(event EventBeginPlay
  (CallFunction|PostPCG)
  (bind _returnvalue (Actor|GetActorOfClass "/Game/Foule/pas_mal/spawning.spawning_C"))
  (Input|EnableInput 0)
  (Components|StaticMesh|SetStaticMesh (Variables|Default|GetStaticMesh) (Variables|Default|GetMesh)))

(event Input|KeyboardEvents|A
  (params (Key :type Key%20Structure :default "None"))
  (:Pressed
    (for (_array_element _array_index) (Variables|/Game/Foule/pas_mal/spawning.spawning_C|GetInsect%20list (stale EventBeginPlay _returnvalue))
      (bind _asia_npc_worm (Utilities|Casting|CastToIA_NPC_worm _array_element))
      (Variables|/Game/Foule/pas_mal/IA_NPC/IA_NPC_worm.IA_NPC_worm_C|Setapple%20location _asia_npc_worm (Utilities|Array|Get(acopy) (Variables|Default|Getworms%20locations) _array_index))
      (Default|CallEat))))

(fn ConstructionScript)

(fn PostPCG
  (params (PCG%20Data :type PCG%20Data%20Collection%20Structure))
  (for (_array_element _array_index) (Actor|GetComponentsByClass "/Script/Engine.InstancedStaticMeshComponent")
    (Components|StaticMesh|SetStaticMesh _array_element "/Game/Foule/pas_mal/worm/worm.worm")
    (Utilities|Array|Add (Variables|Default|Getworms%20locations) (.location (.OutInstanceTransform (Components|InstancedStaticMesh|GetInstanceTransform _array_element _array_index true))))))